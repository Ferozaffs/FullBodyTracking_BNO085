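; BP_Avatar is an avatar Blueprint that reads sensor data over a serial connection.
; BeginPlay opens the port through SerialReader at a fixed port and baud rate, printing a colored success or failure message.
; Each Tick pops the read data, prints every entry, and calls ParseSensorData inside the loop, passing the whole array once per entry rather than the current element.
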(event EventBeginPlay
  ;[1 1 1] Init
  (bind _returnvalue (Class|SerialReader|SetupSerialRead (Variables|Default|GetSerialReader) 6 9600))
  (if _returnvalue
    (Development|PrintString "Success" true true "(R=0.000000,G=1.000000,B=0.182344,A=1.000000)" 1e+01)
    (else
      (Development|PrintString "Failed" true true "(R=1.000000,G=0.005968,B=0.000000,A=1.000000)" 1e+01))))

(event EventTick
  (params (DeltaSeconds :type Float%20%28single-precision%29))
  (bind _returnvalue (Class|SerialReader|PopReadData (Variables|Default|GetSerialReader)))
  (for _array_element _returnvalue
    (Development|PrintString _array_element)
    (Class|Avatar|ParseSensorData self _returnvalue)))

(fn ConstructionScript)